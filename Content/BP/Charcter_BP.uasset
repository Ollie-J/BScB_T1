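; Player character Blueprint whose BeginPlay initializes health and equips a sword.
; It sets Health to MaxHealth, spawns a Sword_BP at the mesh's WeaponSocket and snaps it onto that socket.
; It then prints control hints for movement, sprint, jump and dash as debug strings; the forward-movement hint is unconnected and no input handling appears in this graph.
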(event EventBeginPlay
  (Utilities|FlowControl|Sequence
    (:then_0
      (Variables|Default|SetHealth (Variables|Default|GetMaxHealth))
      (Development|PrintString "health is 100"))
    (:then_1
      ;[0 1 0.1217] Spawning sword due to socket
      (bind _returnvalue (Game|SpawnActorfromClass "/Game/BP/Sword_BP.Sword_BP_C" (Transformation|GetSocketTransform (Variables|Character|GetMesh) "WeaponSocket" "RTS_World") "Undefined" 0 0))
      (Transformation|AttachComponentToComponent _returnvalue (Variables|Character|GetMesh) "WeaponSocket" "SnapToTarget" "SnapToTarget" "SnapToTarget" true))
    (:then_2
      (Development|PrintString "S MoveBack" true true "(R=0.000000,G=0.660000,B=1.000000,A=1.000000)" 1e+04))
    (:then_3
      (Development|PrintString "A Move Left" true true "(R=0.000000,G=0.660000,B=1.000000,A=1.000000)" 1e+04))
    (:then_4
      (Development|PrintString "D Move Right" true true "(R=0.000000,G=0.660000,B=1.000000,A=1.000000)" 1e+04))
    (:then_5
      (Development|PrintString "Left Shift To Sprint" true true "(R=0.000000,G=0.660000,B=1.000000,A=1.000000)" 1e+04))
    (:then_6
      (Development|PrintString "SpaceBar to Jump" true true "(R=0.000000,G=0.660000,B=1.000000,A=1.000000)" 1e+03))
    (:then_7
      (Development|PrintString "E to Dash" true true "(R=0.000000,G=0.660000,B=1.000000,A=1.000000)" 1e+04))))

(fn ConstructionScript)